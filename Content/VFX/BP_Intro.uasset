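; BP_Intro is an intro VFX actor that sets up a black backdrop plane and links to the player GUI's intro slot.
; On BeginPlay it finds the BP_NinjaBase tagged UrActor and stores its widget's NamedSlotIntro in NamedSlots.
; It then applies the black colorizer material to BasePlane and scales it up.
; The construction script sets the asset's trimmed name and path with autonaming.
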(event EventBeginPlay
  (bind _baseplane (Variables|Default|GetBasePlane))
  (Utilities|FlowControl|Sequence
    (:then_0
      ;[0.07596 0.1303 0.2604] Set Widget NamedSlot
      (bind _outactors (Actor|GetAllActorswithTag 0 "UrActor"))
      (bind _asbp_ninja_base (Utilities|Casting|CastToBP_NinjaBase (Utilities|Array|Get(acopy) _outactors)))
      (Variables|Default|SetNamedSlots (Utilities|Array|MakeArray (Variables|/Game/VFX/BP_NinjaGUI.BP_NinjaGUI_C|GetNamedSlot_Intro (Variables|/Game/VFX/BP_NinjaBase.BP_NinjaBase_C|GetBP_Widget_GUI1_Var _asbp_ninja_base)))))
    (:then_1
      (Rendering|Material|SetMaterial _baseplane 0 "/Game/VFX/Core/GUI/MI_ColorizerBlack.MI_ColorizerBlack")
      (Transformation|SetRelativeScale3D _baseplane "45.000000,45.000000,1.000000"))))

(event EventTick
  (params (DeltaSeconds :type Float%20%28single-precision%29)))

(fn ConstructionScript
  (CallFunction|SetAssetTrimmedNameandPath "None" true))