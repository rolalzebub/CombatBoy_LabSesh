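; Runtime control actor that lets the player raise or lower the FluidNinja simulation tick rate with the keyboard.
; On BeginPlay it enables input and seeds its local rate only if CustomTickRate in the default Ninja config DataTable is positive.
; Add and Subtract keys step the clamped rate, print it and write it to TickrateGlobal on the first BP_FluidNinja found.
; The construction script auto-names its editor label.
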(event EventBeginPlay
  ;[0.2448 0.2448 0.2448] Set up local var
  (bind _pickedkeyvalue (CallFunction|DataTableSingleKeyPickerDT "/Game/VFX/DT_NinjaConfig_Default.DT_NinjaConfig_Default" "CustomTickRate"))
  (if (> (Math|Conversions|ToFloat(Integer) _pickedkeyvalue) 0.0)
    (Variables|Default|SetTickRateLocal (Variables|Default|GetTickrate_Global))
    ;[0.2448 0.2448 0.2448] Enable PlayerInput on UrActor
    (Input|EnableInput (Game|GetPlayerController 0))))

(event Input|KeyboardEvents|Add
  (params (Key :type Key%20Structure))
  ;[0.2448 0.2448 0.2448] Define Tickrate
  (:Pressed
    (bind _output_get (Variables|Default|SetTickRateLocal (Math|Float|Clamp(Float) (+ (Variables|Default|GetTickRateLocal) 2e+01) 1.0 5e+02)))
    (Development|PrintString 0 (Utilities|String|Append (Utilities|String|MakeLiteralString "System tick / sec: ") (Utilities|String|ToString(Float) _output_get)) true false "(R=0.018955,G=1.000000,B=0.000000,A=1.000000)" 1.0)
    ;[0.2448 0.2448 0.2448] Set Tickrate On FluidNinja
    (bind _outactors (Actor|GetAllActorsOfClass 0 "/Game/VFX/BP_FluidNinja.BP_FluidNinja_C"))
    (Variables|/Game/VFX/BP_NinjaBase.BP_NinjaBase_C|SetTickrate_Global (Utilities|Array|Get(acopy) _outactors) (Variables|Default|GetTickRateLocal))))

(event Input|KeyboardEvents|Subtract
  (params (Key :type Key%20Structure))
  ;[0.2448 0.2448 0.2448] Define Tickrate
  (:Pressed
    (bind _output_get (Variables|Default|SetTickRateLocal (Math|Float|Clamp(Float) (+ (Variables|Default|GetTickRateLocal) -2e+01) 1.0 5e+02)))
    (Development|PrintString 0 (Utilities|String|Append (Utilities|String|MakeLiteralString "System tick / sec: ") (Utilities|String|ToString(Float) _output_get)) true false "(R=1.000000,G=0.000000,B=0.000000,A=1.000000)" 1.0)
    ;[0.2448 0.2448 0.2448] Set Tickrate On FluidNinja
    (bind _outactors (Actor|GetAllActorsOfClass 0 "/Game/VFX/BP_FluidNinja.BP_FluidNinja_C"))
    (Variables|/Game/VFX/BP_NinjaBase.BP_NinjaBase_C|SetTickrate_Global (Utilities|Array|Get(acopy) _outactors) (Variables|Default|GetTickRateLocal))))

(fn ConstructionScript
  ;[0.1042 0.1042 0.1042 0.755] EditorLabel
  (CallFunction|SetAssetTrimmedNameandPath "None" true))