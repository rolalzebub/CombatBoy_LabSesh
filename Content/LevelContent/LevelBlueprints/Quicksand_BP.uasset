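; Quicksand hazard Blueprint that slows and sinks the player character, restarting the level if they sink too far.
; Entering the Box volume lowers the character's gravity scale, cuts horizontal velocity and sets a slow downward velocity.
; Leaving it restores normal gravity and prints a leftover debug string.
; Overlapping the separate Deathbox volume reloads the current level by name.
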(event OnComponentBeginOverlap(Box)
  (params (OverlappedComponent :type Primitive%20Component%20Object%20Reference) (OtherActor :type Actor%20Object%20Reference) (OtherComp :type Primitive%20Component%20Object%20Reference) (OtherBodyIndex :type Integer) (bFromSweep :type Boolean) (SweepResult :type Hit%20Result%20Structure%20%28by%20ref%29))
  (bind _asmain_player_character_bp (Utilities|Casting|CastToMainPlayer_CharacterBP OtherActor))
  (Variables|/Script/Engine.CharacterMovementComponent|SetGravityScale (Variables|/Script/Engine.Character|GetCharacterMovement _asmain_player_character_bp) 0.1)
  (Variables|/Script/Engine.MovementComponent|SetVelocity (Variables|/Script/Engine.Character|GetCharacterMovement _asmain_player_character_bp) (Math|Vector|MakeVector (/ (.x (Variables|/Script/Engine.MovementComponent|GetVelocity (Variables|/Script/Engine.Character|GetCharacterMovement _asmain_player_character_bp))) 6.0) (/ (.y (Variables|/Script/Engine.MovementComponent|GetVelocity (Variables|/Script/Engine.Character|GetCharacterMovement _asmain_player_character_bp))) 6.0) -5e+01)))

(event OnComponentEndOverlap(Box)
  (params (OverlappedComponent :type Primitive%20Component%20Object%20Reference) (OtherActor :type Actor%20Object%20Reference) (OtherComp :type Primitive%20Component%20Object%20Reference) (OtherBodyIndex :type Integer))
  (bind _asmain_player_character_bp (Utilities|Casting|CastToMainPlayer_CharacterBP OtherActor))
  (Variables|/Script/Engine.CharacterMovementComponent|SetGravityScale (Variables|/Script/Engine.Character|GetCharacterMovement _asmain_player_character_bp) 1.0)
  (Development|PrintString "Hello"))

(event OnComponentBeginOverlap(Deathbox)
  (params (OverlappedComponent :type Primitive%20Component%20Object%20Reference) (OtherActor :type Actor%20Object%20Reference) (OtherComp :type Primitive%20Component%20Object%20Reference) (OtherBodyIndex :type Integer) (bFromSweep :type Boolean) (SweepResult :type Hit%20Result%20Structure%20%28by%20ref%29))
  (Utilities|Casting|CastToMainPlayer_CharacterBP OtherActor)
  (bind _returnvalue (Game|GetCurrentLevelName true))
  (Game|OpenLevel(byName) (Utilities|String|StringToName _returnvalue)))

(fn ConstructionScript)