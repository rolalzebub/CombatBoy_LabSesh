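; AI controller that starts path-following behavior for an AI_Character pawn.
; On BeginPlay it runs PathFollower_BT, caches the controlled pawn and writes that pawn's DesiredNode to the DesiredPathNode blackboard key.
; Tick is empty, and a disconnected branch that would advance along linked NextNode references with MoveToActor based on move status never runs.
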(event EventBeginPlay
  (AI|RunBehaviorTree "/Game/Blueprints/AI/PathFollower_BT.PathFollower_BT")
  (bind _asai_character (Utilities|Casting|CastToAI_Character (Pawn|GetControlledPawn)))
  (bind _output_get (Variables|Default|SetStoredPawn _asai_character))
  (AI|Components|Blackboard|SetValueasObject (AI|GetBlackboard 0) (Variables|Default|GetDesiredPathNode) (Variables|/Game/Blueprints/AI/AI_Character.AI_Character_C|GetDesiredNode _output_get)))

(event EventTick
  (params (DeltaSeconds :type Float%20%28single-precision%29)))

(fn ConstructionScript)