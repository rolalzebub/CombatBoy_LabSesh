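; AI character that detects the player along the Y axis and reports awareness to its Blackboard.
; An awareness sphere sets IsWithinSphere and gates a Tick line trace from the eyes, aimed left or right by capsule yaw.
; A hit sets CanSeePlayer, held by a five-second retriggerable delay, and stores the player's side in BisMovingRight.
; UpdateBlackboard pushes the player reference and seen state.
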(event OnComponentBeginOverlap(Sphere)
  (params (OverlappedComponent :type Primitive%20Component%20Object%20Reference) (OtherActor :type Actor%20Object%20Reference) (OtherComp :type Primitive%20Component%20Object%20Reference) (OtherBodyIndex :type Integer) (bFromSweep :type Boolean) (SweepResult :type Hit%20Result%20Structure%20%28by%20ref%29))
  ;[1 1 1] Is in range of AI Awareness
  (Utilities|Casting|CastToPlayerCharacter OtherActor)
  (Variables|Default|SetIsOverlappingSphere true)
  ;[1 1 1] Currently keeps Ai inactive till within Sphere
  (AI|Components|Blackboard|SetValueasBool (AI|GetBlackboard 0) (Utilities|Name|MakeLiteralName "IsWithinSphere") (Variables|Default|GetIsOverlappingSphere))
  (CallFunction|UpdateBlackboard))

(event OnComponentEndOverlap(Sphere)
  (params (OverlappedComponent :type Primitive%20Component%20Object%20Reference) (OtherActor :type Actor%20Object%20Reference) (OtherComp :type Primitive%20Component%20Object%20Reference) (OtherBodyIndex :type Integer))
  ;[1 1 1] Is in range of AI Awareness
  (Utilities|Casting|CastToPlayerCharacter OtherActor)
  (Variables|Default|SetIsOverlappingSphere false)
  ;[1 1 1] Currently keeps Ai inactive till within Sphere
  (AI|Components|Blackboard|SetValueasBool (AI|GetBlackboard 0) (Utilities|Name|MakeLiteralName "IsWithinSphere") (Variables|Default|GetIsOverlappingSphere))
  (CallFunction|UpdateBlackboard))

(event Custom|SeenPlayerInLast5
  (Variables|Default|SetSeenRecently? true)
  (Utilities|FlowControl|RetriggerableDelay 5.0)
  (Variables|Default|SetSeenRecently? false)
  (CallFunction|UpdateBlackboard))

(event EventTick
  (params (DeltaSeconds :type Float%20%28single-precision%29))
  (bind _eyes (Variables|Default|GetEyes))
  (bind _eyes_2 (Variables|Default|GetEyes))
  (bind _returnvalue (Transformation|GetWorldLocation _eyes))
  (bind _returnvalue_2 (Transformation|GetWorldLocation _eyes_2))
  (if (Variables|Default|GetIsOverlappingSphere)
    ;[1 1 1] Line trace in look direction - Checks if player has been hit
    (if (> (.yaw (Transformation|GetWorldRotation (Variables|Collision|GetCapsuleComponent))) 0.0) ; Looking Left/Right
      (bind _outhit (Collision|LineTraceForObjects _returnvalue_2 (+ _returnvalue_2 "0,500.000000,0.000000") (Variables|Default|GetObject%20Types) false 0 "Persistent"))
      (if (== (.hitactor _outhit) (Variables|Default|GetPlayerRef))
        (Variables|Default|SetSeenRecently? true :!label _label)
        (CallFunction|SeenPlayerinLast5)
        (CallFunction|UpdateBlackboard)
        ;[1 1 1] Checks Players last know direction
        (if (>= (- (.y (Transformation|GetWorldLocation (Variables|/Script/Engine.Character|GetCapsuleComponent (Variables|Default|GetPlayerRef)))) (.y (Transformation|GetWorldLocation (Variables|Collision|GetCapsuleComponent)))) 0.0)
          (Variables|Default|SetbisMovingRight true)
          (else
            (Variables|Default|SetbisMovingRight false))))
      (else
        (bind _outhit_2 (Collision|LineTraceForObjects _returnvalue (- _returnvalue "0,500.000000, 0") (Variables|Default|GetObject%20Types) false 0 "Persistent"))
        (if (== (.hitactor _outhit_2) (Variables|Default|GetPlayerRef))
          (goto _label))))))

(event EventBeginPlay
  (bind _asplayer_character (Utilities|Casting|CastToPlayerCharacter (Game|GetPlayerCharacter 0)))
  (Variables|Default|SetPlayerRef _asplayer_character))

(fn ConstructionScript)

(fn UpdateBlackboard
  (bind _returnvalue (AI|GetBlackboard 0))
  ;[0 0 0] Updates Blackboard with player ref and whether they have been seen recently
  (AI|Components|Blackboard|SetValueasObject _returnvalue (Utilities|Name|MakeLiteralName "PlayerCharacter") (Variables|Default|GetPlayerRef))
  (AI|Components|Blackboard|SetValueasBool _returnvalue (Utilities|Name|MakeLiteralName "CanSeePlayer") (Variables|Default|GetSeenRecently?))
  (return))