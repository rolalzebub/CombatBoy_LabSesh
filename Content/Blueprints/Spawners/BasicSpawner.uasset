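; Spawner actor that keeps one enemy in play, replacing it once its reference is no longer valid.
; From BeginPlay, LoopTillDead polls EnemyToSpawn every five seconds while it is valid.
; When it is invalid, the loop spawns an actor at the Billboard transform, stores it in EnemyToSpawn and restarts.
; The spawn class comes from GetClass on that same invalid reference, with no separate class variable.
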(event Custom|LoopTillDead
  (Utilities|IsValid (Variables|Default|GetEnemyToSpawn) :!label _label
    (:Is%20Valid
      (Utilities|FlowControl|Delay 5.0)
      (goto _label))
    (:Is%20Not%20Valid
      (bind _returnvalue (Game|SpawnActorfromClass (Utilities|GetClass (Variables|Default|GetEnemyToSpawn)) (Transformation|GetWorldTransform (Variables|Default|GetBillboard)) "Undefined" 0 0))
      (Variables|Default|SetEnemyToSpawn _returnvalue)
      (CallFunction|LoopTillDead))))

(event EventBeginPlay
  (CallFunction|LoopTillDead))

(event Collision|EventActorBeginOverlap
  (params (OtherActor :type Actor%20Object%20Reference)))

(event EventTick
  (params (DeltaSeconds :type Float%20%28single-precision%29)))

(fn ConstructionScript)